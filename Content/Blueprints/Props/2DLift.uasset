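; 2D lift prop whose sprite shuttles between its origin and EndLocation.
; An autoplay timeline, rate-scaled by TravelTimeInSeconds, lerps the relative location, then waits StopDelay and runs the opposite way.
; BP_MyCharacter overlapping SafetyCollider triggers timeline play or reverse, intended to move the lift away from the player.
; The construction script applies LiftColor and can preview the end position through TestEndLocation, which resets on BeginPlay.
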(event OnComponentBeginOverlap(SafetyCollider)
  (params (OverlappedComponent :type Primitive%20Component%20Object%20Reference) (OtherActor :type Actor%20Object%20Reference) (OtherComp :type Primitive%20Component%20Object%20Reference) (OtherBodyIndex :type Integer) (bFromSweep :type Boolean) (SweepResult :type Hit%20Result%20Structure%20%28by%20ref%29))
  (bind _lifttimeline (Variables|Default|GetLiftTimeline))
  ;[1 1 1] Overlap Character - Cause Lift to move away from player.
  (Utilities|Casting|CastToBP_MyCharacter OtherActor)
  (if (Components|Activation|IsActive _lifttimeline)
    (if (Audio|Components|Audio|IsPlaying _lifttimeline)
      ;[1 1 1] Handles Lift Movement
      (bind (_direction _lerp_alpha) (Timeline|LiftTimeline Play) ; Autoplay = True
        (:Update
          (Transformation|SetRelativeLocation (Variables|Default|GetLiftSprite) (Math|Vector|Lerp(Vector) "0, 0, 0" (Variables|LiftControls|GetEndLocation) _lerp_alpha) false false))
        (:Finished
          (Utilities|FlowControl|Delay (Variables|LiftControls|GetStopDelay))
          (switch Utilities|FlowControl|Switch|SwitchonETimelineDirection _direction
            (:Forward
              (CallFunction|LiftBackward))
            (:Backward
              (CallFunction|LiftForward)))))
      (else
        (Timeline|LiftTimeline Reverse)))))

(event Custom|LiftForward
  ;[1 1 1] Handles Lift Movement
  (bind (_direction _lerp_alpha) (Timeline|LiftTimeline PlayFromStart) ; Autoplay = True
    (:Update
      (Transformation|SetRelativeLocation (Variables|Default|GetLiftSprite) (Math|Vector|Lerp(Vector) "0, 0, 0" (Variables|LiftControls|GetEndLocation) _lerp_alpha) false false))
    (:Finished
      (Utilities|FlowControl|Delay (Variables|LiftControls|GetStopDelay))
      (switch Utilities|FlowControl|Switch|SwitchonETimelineDirection _direction
        (:Forward
          (CallFunction|LiftBackward))
        (:Backward
          (CallFunction|LiftForward))))))

(event Custom|LiftBackward
  ;[1 1 1] Handles Lift Movement
  (bind (_direction _lerp_alpha) (Timeline|LiftTimeline ReverseFromEnd) ; Autoplay = True
    (:Update
      (Transformation|SetRelativeLocation (Variables|Default|GetLiftSprite) (Math|Vector|Lerp(Vector) "0, 0, 0" (Variables|LiftControls|GetEndLocation) _lerp_alpha) false false))
    (:Finished
      (Utilities|FlowControl|Delay (Variables|LiftControls|GetStopDelay))
      (switch Utilities|FlowControl|Switch|SwitchonETimelineDirection _direction
        (:Forward
          (CallFunction|LiftBackward))
        (:Backward
          (CallFunction|LiftForward))))))

(event EventBeginPlay
  (Components|Timeline|SetPlayRate (Variables|Default|GetLiftTimeline) (/ 1.0 (Variables|LiftControls|GetTravelTimeInSeconds)))
  (Variables|LiftControls|SetTestEndLocation false))

(event Collision|EventActorBeginOverlap
  (params (OtherActor :type Actor%20Object%20Reference)))

(event EventTick
  (params (DeltaSeconds :type Float%20%28single-precision%29)))

(fn ConstructionScript
  (bind _liftsprite (Variables|Default|GetLiftSprite))
  (Transformation|SetRelativeLocation _liftsprite (Math|Vector|SelectVector (Variables|LiftControls|GetEndLocation) "0, 0, 0" (Variables|LiftControls|GetTestEndLocation)) false false)
  (Sprite|SetSpriteColor _liftsprite (Variables|LiftControls|GetLiftColor)))