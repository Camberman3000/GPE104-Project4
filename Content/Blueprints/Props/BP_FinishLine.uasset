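; BP_FinishLine is a level goal prop that ends the game in a win when the player character enters its box.
; BeginPlay caches the BP_PlayerController reference.
; On overlap it sets that controller's GameWon flag before the character cast, so any overlapping actor sets it.
; For BP_MyCharacter it then prints a win message, plays a fanfare, waits briefly, shows the MainMenu widget and pauses the game.
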(event OnComponentBeginOverlap(Box)
  (params (OverlappedComponent :type Primitive%20Component%20Object%20Reference) (OtherActor :type Actor%20Object%20Reference) (OtherComp :type Primitive%20Component%20Object%20Reference) (OtherBodyIndex :type Integer) (bFromSweep :type Boolean) (SweepResult :type Hit%20Result%20Structure%20%28by%20ref%29))
  (Variables|/Game/Blueprints/Player/BP_PlayerController.BP_PlayerController_C|SetGameWon? (Variables|References|GetPlayerControllerRef) true)
  (Utilities|Casting|CastToBP_MyCharacter OtherActor)
  (Development|PrintString "YOU WON!")
  (Audio|PlaySound2D "/Game/Sounds/tada.tada" 1.0 1.0 0.0 0 0)
  (Utilities|FlowControl|Delay 0.5)
  (bind _returnvalue (UserInterface|CreateWidget "/Game/Blueprints/UI/MainMenu.MainMenu_C"))
  (UserInterface|Viewport|AddtoViewport _returnvalue 0)
  (Game|SetGamePaused true))

(event EventBeginPlay
  (bind _asbp_player_controller (Utilities|Casting|CastToBP_PlayerController (Game|GetPlayerController 0)))
  (Variables|References|SetPlayerControllerRef _asbp_player_controller))

(event Collision|EventActorBeginOverlap
  (params (OtherActor :type Actor%20Object%20Reference)))

(event EventTick
  (params (DeltaSeconds :type Float%20%28single-precision%29)))

(fn ConstructionScript)