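; Enemy actor that reacts to the player through two overlap spheres, warning at range and dealing damage up close.
; The danger sphere speeds up animation, plays a sound and flips the movement component's Reverse flag unless actor and player control yaws match exactly.
; The attack sphere pauses movement and damages once until CanAttack resets on danger-sphere exit or respawn.
; On death, it destroys the player, then spawns and possesses a new character at the first PlayerStart.
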(event OnComponentBeginOverlap(DangerSphere)
  (params (OverlappedComponent :type Primitive%20Component%20Object%20Reference) (OtherActor :type Actor%20Object%20Reference) (OtherComp :type Primitive%20Component%20Object%20Reference) (OtherBodyIndex :type Integer) (bFromSweep :type Boolean) (SweepResult :type Hit%20Result%20Structure%20%28by%20ref%29))
  ;[1 1 1] Danger Sphere overlap
  (bind _asbp_my_character (Utilities|Casting|CastToBP_MyCharacter OtherActor))
  (Variables|Default|SetPlayerCharRef _asbp_my_character)
  (CallFunction|RotateEnemytoFacePlayer _asbp_my_character)
  (Development|PrintString "DANGER!!")
  (CallFunction|SetEnemyAnimFast)
  (CallFunction|PlayDangerSound (Variables|Default|GetDangerSoundToPlay)))

(event OnComponentBeginOverlap(AttackSphere)
  (params (OverlappedComponent :type Primitive%20Component%20Object%20Reference) (OtherActor :type Actor%20Object%20Reference) (OtherComp :type Primitive%20Component%20Object%20Reference) (OtherBodyIndex :type Integer) (bFromSweep :type Boolean) (SweepResult :type Hit%20Result%20Structure%20%28by%20ref%29))
  (bind _dangersoundref (Variables|EnemyInfo|GetDangerSoundRef))
  ;[1 1 1] Attack Sphere Overlap
  (bind _asbp_my_character (Utilities|Casting|CastToBP_MyCharacter OtherActor))
  (Variables|Default|SetPlayerCharRef _asbp_my_character)
  (Utilities|IsValid _dangersoundref
    (:Is%20Valid
      (Audio|Components|Audio|Stop _dangersoundref))
    (:Is%20Not%20Valid
      _))
  (if (Variables|Default|GetCanAttack?)
    (Variables|Default|SetCanAttack? false)
    (Development|PrintString "I'M HIT. OW!")
    (Utilities|Time|PauseTimerbyHandle (Variables|/Game/Blueprints/BPC_EnemyMovement.BPC_EnemyMovement_C|GetTimerRef (Variables|Default|GetBPC_EnemyMovement)))
    (CallFunction|PlayDangerSound (Variables|Default|GetAttackSoundToPlay))
    (bind _outputpin (Utilities|UpdatePlayerHealth)
      (:PlayerDead
        (Actor|DestroyActor _outputpin)
        (CallFunction|StopSound (Variables|EnemyInfo|GetDangerSoundRef))
        (CallFunction|SetEnemyAnimNormal)
        (CallFunction|RespawnPlayer)))))

(event OnComponentEndOverlap(DangerSphere)
  (params (OverlappedComponent :type Primitive%20Component%20Object%20Reference) (OtherActor :type Actor%20Object%20Reference) (OtherComp :type Primitive%20Component%20Object%20Reference) (OtherBodyIndex :type Integer))
  ;[1 1 1] Danger Sphere overlap
  (Utilities|Casting|CastToBP_MyCharacter OtherActor)
  (Components|Timeline|SetPlayRate (Variables|Default|Getanimation) 1.0)
  (Variables|Default|SetCanAttack? true)
  (CallFunction|StopSound (Variables|EnemyInfo|GetDangerSoundRef)))

(event OnComponentEndOverlap(AttackSphere)
  (params (OverlappedComponent :type Primitive%20Component%20Object%20Reference) (OtherActor :type Actor%20Object%20Reference) (OtherComp :type Primitive%20Component%20Object%20Reference) (OtherBodyIndex :type Integer))
  ;[1 1 1] Attack Sphere Overlap
  (Utilities|Casting|CastToBP_MyCharacter OtherActor)
  (Utilities|Time|UnpauseTimerbyHandle (Variables|/Game/Blueprints/BPC_EnemyMovement.BPC_EnemyMovement_C|GetTimerRef (Variables|Default|GetBPC_EnemyMovement)))
  (Components|Timeline|SetPlayRate (Variables|Default|Getanimation) 1.0))

(event EventBeginPlay
  (bind _asbp_my_character (Utilities|Casting|CastToBP_MyCharacter (Game|GetPlayerCharacter 0)))
  (Variables|Default|SetPlayerCharRef _asbp_my_character))

(fn ConstructionScript)

(fn StopSound
  (params (Target :type Audio%20Component%20Object%20Reference))
  (Utilities|IsValid Target
    (:Is%20Valid
      (Audio|Components|Audio|Stop Target))))

(fn SetEnemyAnimNormal
  (Components|Timeline|SetPlayRate (Variables|Default|Getanimation) 1.0))

(fn SetEnemyAnimFast
  (Components|Timeline|SetPlayRate (Variables|Default|Getanimation) 1e+01))

(fn RespawnPlayer
  (bind _outactors (Actor|GetAllActorsOfClass "/Script/Engine.PlayerStart"))
  (bind _returnvalue (Game|SpawnActorfromClass "/Game/Blueprints/BP_MyCharacter.BP_MyCharacter_C" (Math|Transform|MakeTransform (Transformation|GetActorLocation (Utilities|Array|Get(acopy) _outactors)) "0, 0, 0" "1,1,1") "Undefined" 0 0))
  (Pawn|Possess (Game|GetPlayerController 0) _returnvalue)
  (Variables|/Game/Blueprints/BP_MyCharacter.BP_MyCharacter_C|SetHealth _returnvalue 1e+02)
  (Variables|Default|SetCanAttack? true))

(fn PlayDangerSound
  (params (Sound :type Sound%20Base%20Object%20Reference))
  (bind _returnvalue (Audio|SpawnSound2D Sound 1.0 1.0 0.0 0))
  (Utilities|IsValid (Variables|EnemyInfo|GetDangerSoundRef)
    (:Is%20Not%20Valid
      (Variables|EnemyInfo|SetDangerSoundRef _returnvalue))))

(fn RotateEnemytoFacePlayer
  (params (self2 :type Pawn%20Object%20Reference))
  (bind _bpc_enemymovement (Variables|Default|GetBPC_EnemyMovement))
  (if (== (.Yaw (Math|Rotator|BreakRotator (Transformation|GetActorRotation))) (.Yaw (Math|Rotator|BreakRotator (Pawn|GetControlRotation self2 :!class /Script/Engine.Pawn)))) ; Facing player?
    (Development|PrintString "Facing Player")
    (else
      (Development|PrintString "NOT facing player")
      (if (Variables|/Game/Blueprints/BPC_EnemyMovement.BPC_EnemyMovement_C|GetReverse? _bpc_enemymovement)
        (Variables|/Game/Blueprints/BPC_EnemyMovement.BPC_EnemyMovement_C|SetReverse? _bpc_enemymovement false)
        (else
          (Variables|/Game/Blueprints/BPC_EnemyMovement.BPC_EnemyMovement_C|SetReverse? _bpc_enemymovement true)))))
  (return))

(fn PlayAttackSound
  (params (Sound :type Sound%20Base%20Object%20Reference))
  (bind _returnvalue (Audio|SpawnSound2D Sound 1.0 1.0 0.0 0))
  (Utilities|IsValid _returnvalue
    (:Is%20Not%20Valid
      (Variables|EnemyInfo|SetAttackSoundRef _returnvalue))))