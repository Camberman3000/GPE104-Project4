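; BP_Bee is a bee enemy that menaces and attacks the player through two overlap spheres, delegating to movement, animation, sound and attack components.
; The danger sphere turns it toward the player, speeds up animation and plays a warning sound.
; The attack sphere pauses the movement timer and updates player health, destroying and respawning the player when that returns true.
; A CanAttack flag blocks repeat hits until danger-sphere exit or respawn.
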(event OnComponentBeginOverlap(DangerSphere)
  (params (OverlappedComponent :type Primitive%20Component%20Object%20Reference) (OtherActor :type Actor%20Object%20Reference) (OtherComp :type Primitive%20Component%20Object%20Reference) (OtherBodyIndex :type Integer) (bFromSweep :type Boolean) (SweepResult :type Hit%20Result%20Structure%20%28by%20ref%29))
  ;[1 0.8922 0] Danger Sphere overlap
  (CallFunction|HandleDangerOverlap OtherActor))

(event OnComponentBeginOverlap(AttackSphere)
  (params (OverlappedComponent :type Primitive%20Component%20Object%20Reference) (OtherActor :type Actor%20Object%20Reference) (OtherComp :type Primitive%20Component%20Object%20Reference) (OtherBodyIndex :type Integer) (bFromSweep :type Boolean) (SweepResult :type Hit%20Result%20Structure%20%28by%20ref%29))
  ;[1 0 0] Attack Sphere Overlap
  (CallFunction|HandleAttackOverlap OtherActor))

(event OnComponentEndOverlap(DangerSphere)
  (params (OverlappedComponent :type Primitive%20Component%20Object%20Reference) (OtherActor :type Actor%20Object%20Reference) (OtherComp :type Primitive%20Component%20Object%20Reference) (OtherBodyIndex :type Integer))
  ;[1 0.8922 0] Danger Sphere overlap
  (CallFunction|HandleDangerEndOverlap OtherActor))

(event OnComponentEndOverlap(AttackSphere)
  (params (OverlappedComponent :type Primitive%20Component%20Object%20Reference) (OtherActor :type Actor%20Object%20Reference) (OtherComp :type Primitive%20Component%20Object%20Reference) (OtherBodyIndex :type Integer))
  ;[1 0 0] Attack Sphere Overlap
  (CallFunction|HandleAttackOverlapEnd OtherActor))

(event EventBeginPlay
  (bind _asbp_my_character (Utilities|Casting|CastToBP_MyCharacter (Game|GetPlayerCharacter 0)))
  (Variables|References|SetPlayerCharRef _asbp_my_character)
  (bind _asbp_player_controller (Utilities|Casting|CastToBP_PlayerController (Game|GetPlayerController 0)))
  (Variables|References|SetPlayerControllerRef _asbp_player_controller))

(fn ConstructionScript)

(fn HandleDangerOverlap
  (params (Object :type Object%20Object%20Reference))
  (bind _asbp_my_character (Utilities|Casting|CastToBP_MyCharacter Object))
  (bind _output_get (Variables|References|SetPlayerCharRef _asbp_my_character))
  (Default|RotateEnemytoFacePlayer (Variables|Default|GetBPC_EnemyMovement) _output_get)
  (Default|SetEnemyAnimSpeed (Variables|Default|GetBPC_EnemyAnimation) (Variables|EnemyInfo|GetAnimFastSpeed))
  (Default|PlaySound (Variables|Default|GetBPC_EnemySounds) (Variables|EnemyInfo|GetDangerSoundToPlay)))

(fn HandleDangerEndOverlap
  (params (Object :type Object%20Object%20Reference))
  (Utilities|Casting|CastToBP_MyCharacter Object)
  (Default|SetEnemyAnimSpeed (Variables|Default|GetBPC_EnemyAnimation) (Variables|EnemyInfo|GetAnimSlowSpeed))
  (Variables|Default|SetCanAttack? true)
  (Default|StopSound (Variables|Default|GetBPC_EnemySounds) (Variables|/Game/Blueprints/Enemy/BPC_EnemySounds.BPC_EnemySounds_C|GetSoundRef (Variables|Default|GetBPC_EnemySounds))))

(fn HandleAttackOverlap
  (params (Object :type Object%20Object%20Reference))
  (bind _bpc_enemysounds (Variables|Default|GetBPC_EnemySounds))
  (bind _asbp_my_character (Utilities|Casting|CastToBP_MyCharacter Object))
  (Variables|References|SetPlayerCharRef _asbp_my_character)
  (if (Variables|Default|GetCanAttack?)
    (Variables|Default|SetCanAttack? false)
    (Development|PrintString "I'M HIT. OW!")
    (Utilities|Time|PauseTimerbyHandle (Variables|/Game/Blueprints/Enemy/BPC_EnemyMovement.BPC_EnemyMovement_C|GetTimerRef (Variables|Default|GetBPC_EnemyMovement)))
    (Default|StopSound _bpc_enemysounds (Variables|/Game/Blueprints/Enemy/BPC_EnemySounds.BPC_EnemySounds_C|GetSoundRef _bpc_enemysounds)) ; Stop Danger sound
    (Default|PlaySound (Variables|Default|GetBPC_EnemySounds) (Variables|EnemyInfo|GetAttackSoundToPlay))
    (bind _dead_ (Default|UpdatePlayerHealth (Variables|Default|GetBPC_EnemyAttack)))
    (if _dead_
      (Actor|DestroyActor (Variables|References|GetPlayerCharRef))
      (Default|RespawnPlayer (Variables|References|GetPlayerControllerRef))
      (Variables|Default|SetCanAttack? true)
      (else
        (Default|SetEnemyAnimSpeed (Variables|Default|GetBPC_EnemyAnimation) (Variables|EnemyInfo|GetAnimSlowSpeed))))))

(fn HandleAttackOverlapEnd
  (params (Object :type Object%20Object%20Reference))
  (Utilities|Casting|CastToBP_MyCharacter Object)
  (Utilities|Time|UnpauseTimerbyHandle (Variables|/Game/Blueprints/Enemy/BPC_EnemyMovement.BPC_EnemyMovement_C|GetTimerRef (Variables|Default|GetBPC_EnemyMovement)))
  (Default|SetEnemyAnimSpeed (Variables|Default|GetBPC_EnemyAnimation) (Variables|EnemyInfo|GetAnimSlowSpeed)))