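; Enemy attack component for BP_Bee that provides two events for knocking the player off a platform.
; BeginPlay caches the owning bee, the player character and the player controller.
; DropPlayerThroughPlatform turns off collision on the game mode's SawPlatform, then restores it after a one-second delay.
; TeleportPlayerOffPlatform shifts the player along X by a variable plus a fixed offset, keeping Y and Z.
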(event Custom|DropPlayerThroughPlatform
  ;[1 0.6094 0] Drop Player Through Platform
  (bind _asbp_game_mode (Utilities|Casting|CastToBP_GameMode (Game|GetGameMode)))
  (Collision|SetCollisionEnabled (Variables|/Script/Paper2D.PaperSpriteActor|GetRenderComponent (Variables|/Game/Blueprints/BP_GameMode.BP_GameMode_C|GetSawPlatform _asbp_game_mode)) "NoCollision")
  (Utilities|FlowControl|Delay 1.0)
  (Collision|SetCollisionEnabled (Variables|/Script/Paper2D.PaperSpriteActor|GetRenderComponent (Variables|/Game/Blueprints/BP_GameMode.BP_GameMode_C|GetSawPlatform _asbp_game_mode)) "QueryAndPhysics"))

(event Custom|TeleportPlayerOffPlatform
  ;[1 0 0.9375] Teleport Player Off Platform
  (bind _asbp_my_character (Utilities|Casting|CastToBP_MyCharacter (Game|GetPlayerCharacter 0)))
  (Variables|References|SetPlayerCharRef _asbp_my_character)
  (Variables|Default|SetOrigPlayerLocation (Transformation|GetActorLocation (Variables|References|GetPlayerCharRef)))
  (Transformation|SetActorTransform (Variables|References|GetPlayerCharRef) (Math|Transform|MakeTransform (Math|Vector|MakeVector (- (.X (Math|Vector|BreakVector (Variables|Default|GetOrigPlayerLocation))) (+ (Variables|Default|GetPlayerNewX) 7.5e+02)) (.Y (Math|Vector|BreakVector (Variables|Default|GetOrigPlayerLocation))) (.Z (Math|Vector|BreakVector (Variables|Default|GetOrigPlayerLocation)))) "0, 0, 0" "1,1,1")))

(event EventBeginPlay
  (bind _asbp_bee (Utilities|Casting|CastToBP_Bee (Components|GetOwner)))
  (Variables|References|SetEnemyRef _asbp_bee)
  (bind _asbp_my_character (Utilities|Casting|CastToBP_MyCharacter (Game|GetPlayerCharacter 0)))
  (Variables|References|SetPlayerCharRef _asbp_my_character)
  (bind _asbp_player_controller (Utilities|Casting|CastToBP_PlayerController (Game|GetPlayerController 0)))
  (Variables|References|SetPlayerControllerRef _asbp_player_controller))

(event EventTick
  (params (DeltaSeconds :type Float%20%28single-precision%29)))