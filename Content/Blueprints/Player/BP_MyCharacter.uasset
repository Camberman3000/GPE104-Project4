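; Player character for a 2D side-scroller with horizontal movement, double jump and flipbook animation.
; The MoveRight axis drives movement, turns the controller's yaw to face the travel direction and triggers animation updates.
; A DoN gate allows a normal jump then a launch, resetting on landing.
; AnimationStateMachine picks idle, run or jump flipbooks from velocity and falling state; the sprite component is set to replicate.
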(event Custom|UpdateAnimation
  ;[0.4531 1 0] Animation handling
  (Variables|Default|SetIsMoving? (> (Math|Vector|VectorLength (Transformation|GetVelocity)) 0.0))
  (Variables|Default|SetIsFalling? (AI|Components|NavMovement|IsFalling (Variables|Character|GetCharacterMovement)))
  (bind _outflipbook (CallFunction|AnimationStateMachine (Variables|Default|GetIsFalling?) (Variables|Default|GetIsMoving?)))
  (Sprite|SetFlipbook (Variables|Default|GetSprite) _outflipbook))

(event EventBeginPlay
  ;[0 1 0.08594] Replication
  (Class|ActorComponent|SetIsReplicated (Variables|Default|GetSprite) true))

(event Collision|EventActorBeginOverlap
  (params (OtherActor :type Actor%20Object%20Reference)))

(event EventTick
  (params (DeltaSeconds :type Float%20%28single-precision%29)))

(event EventOnLanded
  (params (Hit :type Hit%20Result%20Structure%20%28by%20ref%29))
  ;[1 0 0.5625] Jump - 1 press for single jump and 2 for double - Resets upon landing
  (Utilities|FlowControl|DoN 2) ; enters at Reset
)

(event Input|ActionEvents|InputActionJump
  (params (Key :type Key%20Structure :default "None"))
  ;[1 0 0.5625] Jump - 1 press for single jump and 2 for double - Resets upon landing
  (:Pressed
    (bind _counter (Utilities|FlowControl|DoN 2)
      (:Exit
        (switch int _counter
          (:1
            (Character|Jump))
          (:2
            (Character|LaunchCharacter (Math|Vector|MakeVector 0.0 0.0 (Variables|Default|GetLaunchVelocity)) false false)))))))

(event Input|AxisEvents|InputAxisMoveRight
  (params (AxisValue :type Float%20%28single-precision%29))
  ;[1 0.8438 0] Movement
  (Pawn|Input|AddMovementInput "1.000000, 0, 0" AxisValue false)
  (CallFunction|UpdateAnimation)
  (Math|Float|CompareFloat AxisValue 0.0
    (:>
      (Pawn|SetControlRotation (Pawn|GetController) (Math|Rotator|MakeRotator 0.0 0.0 0.0)))
    (:<
      (Pawn|SetControlRotation (Pawn|GetController) (Math|Rotator|MakeRotator 0.0 0.0 1.8e+02)))))

(fn ConstructionScript)

(fn AnimationStateMachine
  (params (IsFalling? :type Boolean) (IsMoving? :type Boolean))
  (LocalVariables|SetL_Falling IsFalling?)
  (LocalVariables|SetL_Moving IsMoving?)
  (if (LocalVariables|GetL_Falling)
    (LocalVariables|SetL_EAnimationState "NewEnumerator2")
    (elif (LocalVariables|GetL_Moving)
      (LocalVariables|SetL_EAnimationState "NewEnumerator1")
      (else
        (LocalVariables|SetL_EAnimationState "NewEnumerator0"))))
  (return (Utilities|Select :Index (LocalVariables|GetL_EAnimationState) :NewEnumerator0 (Variables|Animations|GetIdleFlipbook) :NewEnumerator1 (Variables|Animations|GetRunFlipbook) :NewEnumerator2 (Variables|Animations|GetJumpFlipbook))))